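; Gameplay ability that, by its name and folder, is a passive startup listener for gameplay events; its Blueprint ActivateAbility does nothing.
; GetModuleName returns a script module path for the ability.
; An unconnected, never-run graph waits for Attributes events and applies EventBasedEffectClass to self, passing the magnitude by SetByCaller to the matching tag and zeroing other EventTags.
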(event Ability|EventActivateAbility)

(fn GetModuleName
  (return "Blueprints.AbilitySystem.Aura.Abilities.Passive_Startup.GA_ListenForEvent"))