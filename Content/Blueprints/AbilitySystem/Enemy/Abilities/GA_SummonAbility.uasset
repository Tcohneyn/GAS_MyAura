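; GA_SummonAbility is an enemy gameplay ability for summoning minions, bound to a script module through GetModuleName.
; Its Blueprint events are empty, so none of the summoning graph runs here.
; Disconnected nodes sketch shuffled spawn locations, a summon effect, a montage with gameplay event wait, minion spawning with default controllers, and a destroyed-callback binding.
; The returned module path suggests the live logic is in script, likely UnLua.
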(event Custom|OnMinionDestroyed
  (params (DestroyedActor :type Actor%20Object%20Reference)))

(event Ability|EventActivateAbility)

(event Ability|EventOnEndAbility
  (params (bWasCancelled :type Boolean)))

(fn GetModuleName
  (return "Blueprints.AbilitySystem.Enemy.Abilities.GA_SummonAbility"))